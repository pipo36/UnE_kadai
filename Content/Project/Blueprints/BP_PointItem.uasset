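; BP_PointItem is a collectible actor that awards points to whatever overlaps its box.
; The construction script looks up its row in DT_PointItem to set the point value and mesh material.
; A Rotate timeline spins the mesh around yaw.
; On overlap, it sends its name and points to the other actor through the CharacterHitActionMessage call, plays a sound and destroys itself.
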(event `self.ReceiveBeginPlay`
  (bind (_direction _rotation) (`Timeline|Rotate`)
    (:`Update`
      (if (< (`self.ActorRotation`) 360.0)
        (set `self.ActorRotation` _rotation)
        (else
          (set `self.ActorRotation` 0.0)))
      (`SceneComponent.K2_SetRelativeRotation` (`self.STM_PointItem`) (`KismetMathLibrary.MakeRotator` 0.0 0.0 (`self.ActorRotation`)) false false))))

(event `self.Box.OnComponentBeginOverlap`
  (params (OverlappedComponent :type "PrimitiveComponent Object Reference") (OtherActor :type "Actor Object Reference") (OtherComp :type "PrimitiveComponent Object Reference") (OtherBodyIndex :type Integer) (bFromSweep :type Boolean) (SweepResult :type "HitResult Structure (by ref)"))
  (message `/Game/Project/Blueprints/BPI_MyCharacter.CharacterHitAction` OtherActor (`KismetSystemLibrary.GetDisplayName` self) (`self.Point`))
  (`GameplayStatics.PlaySoundAtLocation` "/Game/Game_Item/Pick_Up/Wav/Wav_Ashorttactilesou1_wav.Wav_Ashorttactilesou1_wav" (`self.K2_GetActorLocation`) (struct) 1.0 1.0 0.0 null null null null)
  (`self.K2_DestroyActor`))

(fn `UserConstructionScript`
  (bind _returnvalue (`|GetDataTableRow` "/Game/Project/Blueprints/DT_PointItem.DT_PointItem" (`self.PointItemDataName`))
    (:`then`
      (bind (_point _material) (break `/Game/Project/Blueprints/ST_PointItem` _returnvalue))
      (set `self.Point` _point)
      (`PrimitiveComponent.SetMaterial` (`self.STM_PointItem`) 0 _material))))